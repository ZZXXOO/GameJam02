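; Game state Blueprint that runs a road-by-road game loop with scoring.
; NextRoad starts the random spawner, sends the AI character along the road picked by RoadIndex, then increments the index.
; ArrivePoint stops spawning, awards points and shows a station widget, or the end-game menu after the third road despite five mapped.
; AddScoreValue multiplies points by RoadIndex, so arrival bonuses scale with its square, and updates the score UI.
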(event Custom|NextRoad
  (bind _tpm_bp (Variables|Default|GetTPM_BP))
  (bind _aicharacter (Variables|Default|GetAICharacter))
  (Default|StartSpawn (Variables|Default|GetRandomSpawnBP))
  (Variables|/Game/AI_Character.AI_Character_C|SetMovePointActor _aicharacter (Utilities|Select :Index (Variables|Default|GetRoadIndex) :Option%200 (Variables|/Game/BP_TargetPointManger.BP_TargetPointManger_C|GetRoad1 _tpm_bp) :Option%201 (Variables|/Game/BP_TargetPointManger.BP_TargetPointManger_C|GetRoad2 _tpm_bp) :Option%202 (Variables|/Game/BP_TargetPointManger.BP_TargetPointManger_C|GetRoad3 _tpm_bp) :Option%203 (Variables|/Game/BP_TargetPointManger.BP_TargetPointManger_C|GetRoad4 _tpm_bp) :Option%204 (Variables|/Game/BP_TargetPointManger.BP_TargetPointManger_C|GetRoad5 _tpm_bp)))
  (Default|StartMove _aicharacter)
  (Math|Integer|IncrementInt (Variables|Default|GetRoadIndex)))

(event Custom|AddScoreValue
  (params (AddValue :type Integer))
  (Variables|Default|SetScoreValue (+ (Variables|Default|GetScoreValue) (* AddValue (Variables|Default|GetRoadIndex))))
  (Default|UpdataScore (Variables|Default|GetUIScore) (Variables|Default|GetScoreValue)))

(event Custom|ArrivePoint
  (Default|StopSpawn (Variables|Default|GetRandomSpawnBP))
  (CallFunction|AddScoreValue (* (Variables|Default|GetRoadIndex) 100))
  (if (== (Variables|Default|GetRoadIndex) 3)
    (bind _returnvalue (UserInterface|CreateWidget "/Game/UI/UI_EndGameMenu.UI_EndGameMenu_C"))
    (UserInterface|Viewport|AddtoViewport _returnvalue 0)
    (else
      (bind _returnvalue_2 (UserInterface|CreateWidget "/Game/UI/UI_PointStation.UI_PointStation_C"))
      (UserInterface|Viewport|AddtoViewport _returnvalue_2 0))))

(event EventBeginPlay)

(event EventTick
  (params (DeltaSeconds :type Float%20%28single-precision%29)))

(fn ConstructionScript)