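; BP_RandomSpawn is a spawner that keeps creating BP_FlyFruits actors ahead of the AI character.
; On BeginPlay it caches the first AI_Character found, then after a short delay enters an endless delay-driven loop that spawns a fruit every two seconds.
; Each scaled-up fruit appears at a random forward and sideways offset from the character's current location and facing, and always spawns regardless of collision.
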(event EventBeginPlay
  (bind _outactors (Actor|GetAllActorsOfClass "/Game/AI_Character.AI_Character_C"))
  (Variables|Default|SetAICharacter (Utilities|Array|Get(acopy) _outactors))
  (Utilities|FlowControl|Delay 0.5)
  (Game|SpawnActorfromClass "/Game/WMJ/BP_FlyFruits.BP_FlyFruits_C" (Math|Transform|MakeTransform (+ (+ (Transformation|GetActorLocation (Variables|Default|GetAICharacter)) (* (Transformation|GetActorForwardVector (Variables|Default|GetAICharacter)) (Math|Random|RandomFloatinRange 4e+02 1e+03))) (* (Transformation|GetActorRightVector (Variables|Default|GetAICharacter)) (Math|Random|RandomFloatinRange -1e+03 1e+03))) "0, 0, 0" "3.000000,3.000000,3.000000") "AlwaysSpawn" 0 0 :!label _label)
  (Utilities|FlowControl|Delay 2.0)
  (goto _label))

(fn ConstructionScript)