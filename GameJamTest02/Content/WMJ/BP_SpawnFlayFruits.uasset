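; Spawner actor that periodically creates BP_FlyFruits actors around the player pawn.
; BeginPlay starts a looping timer with an interval randomized once, then immediately runs a first spawn burst.
; The timer event re-enters the same spawn loop, placing a random number of fruits at random X/Y offsets near the pawn, at its height.
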(event Custom|Spawn_Actor
  (bind _returnvalue (Game|Player|GetPlayerPawn 0))
  (bind _returnvalue_2 (Transformation|GetActorLocation _returnvalue))
  (for _index (range 0 (Math|Random|RandomIntegerinRange 0 4))
    (Game|SpawnActorfromClass "/Game/WMJ/BP_FlyFruits.BP_FlyFruits_C" (Math|Conversions|ToTransform(Vector) (Math|Vector|MakeVector (Math|Random|RandomFloatinRange (- (.x _returnvalue_2) 5e+01) (+ (.x _returnvalue_2) 5e+01)) (Math|Random|RandomFloatinRange (- (.y _returnvalue_2) 5e+01) (+ (.y _returnvalue_2) 5e+01)) (.z _returnvalue_2))) "Undefined" 0 0)))

(event EventBeginPlay
  (bind _returnvalue (Game|Player|GetPlayerPawn 0))
  (bind _returnvalue_2 (Transformation|GetActorLocation _returnvalue))
  (Utilities|FlowControl|Sequence
    (:then_0
      (Utilities|Time|SetTimerbyEvent (delegate Custom|Spawn_Actor) (Math|Random|RandomFloatinRange 2.0 5.0) true))
    (:then_1
      (for _index (range 0 (Math|Random|RandomIntegerinRange 0 4))
        (Game|SpawnActorfromClass "/Game/WMJ/BP_FlyFruits.BP_FlyFruits_C" (Math|Conversions|ToTransform(Vector) (Math|Vector|MakeVector (Math|Random|RandomFloatinRange (- (.x _returnvalue_2) 5e+01) (+ (.x _returnvalue_2) 5e+01)) (Math|Random|RandomFloatinRange (- (.y _returnvalue_2) 5e+01) (+ (.y _returnvalue_2) 5e+01)) (.z _returnvalue_2))) "Undefined" 0 0)))))

(fn ConstructionScript)