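; Flying fruit actor that picks a random mesh and flies it toward a randomized point near screen center, in front of the camera.
; A timeline drives the flight through screen deprojection, then enables physics, with a random chance of an impulse and delayed destruction.
; Clicking stops the flight and drags the actor under the cursor, except two mesh indices, which open UI_Cake and destroy it.
; Mouse release drops picked fruits back into physics.
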(event OnClicked(ST_Fruits)
  (params (TouchedComponent :type Primitive%20Component%20Object%20Reference) (ButtonPressed :type Key%20Structure :default "None"))
  (bind _st_index (Variables|Default|GetSt_Index))
  (Variables|Default|SetCan_Pick? true)
  (Development|PrintString (Utilities|String|ToString(Integer) _st_index))
  (if (or (== _st_index 1) (== _st_index 2))
    (bind _returnvalue (UserInterface|CreateWidget "/Game/WMJ/UI_Cake.UI_Cake_C"))
    (UserInterface|Viewport|AddtoPlayerScreen _returnvalue)
    (Actor|DestroyActor)
    (else
      (Physics|SetSimulatePhysics (Variables|Default|GetST_Fruits) false)
      (CallFunction|StopTime))))

(event OnReleased(ST_Fruits)
  (params (TouchedComponent :type Primitive%20Component%20Object%20Reference) (ButtonReleased :type Key%20Structure :default "None"))
  (CallFunction|DropActor))

(event Custom|Stop_Time
  (bind _returnvalue (Viewport|GetViewportSize))
  (bind _returnvalue_2 (Game|GetPlayerController 0))
  (bind _st_fruits (Variables|Default|GetST_Fruits))
  (bind _random_floatx (Variables|Default|GetRandom_FloatX))
  (bind _random_floaty (Variables|Default|GetRandom_FloatY))
  (bind _returnvalue_3 (/ _returnvalue 2.0))
  (bind _returnvalue_4 (+ (.y _returnvalue_3) _random_floaty))
  (bind _returnvalue_5 (+ (.x _returnvalue_3) _random_floatx))
  (bind (_worldposition _worlddirection) (Class|GameplayStatics|DeprojectScreentoWorld _returnvalue_2 (Math|Vector2D|MakeVector2D _returnvalue_5 _returnvalue_4)))
  (bind _returnvalue_6 (* _worlddirection 1e+02))
  (bind _returnvalue_7 (+ _worldposition _returnvalue_6))
  (bind _新建轨迹_0 (Timeline|时间轴_0 Stop)
    (:Update
      (Transformation|SetWorldLocation (Variables|Default|GetST_Fruits) (Math|Vector|Lerp(Vector) (Transformation|GetActorLocation) _returnvalue_7 _新建轨迹_0) false false))
    (:Finished
      (Variables|/Script/Engine.RotatingMovementComponent|SetRotationRate (Variables|Default|GetRotatingMovement) "0, 0, 0")
      (Physics|SetSimulatePhysics _st_fruits true)
      (if (not (Math|Conversions|ToBoolean(Integer) (Math|Random|RandomIntegerinRange 0 1)))
        (Physics|AddImpulse _st_fruits (* _returnvalue_7 1.0) "None" false)
        (Utilities|FlowControl|Delay 2.0)
        (Actor|DestroyActor)))))

(event Custom|Drop_Actor
  (if (Variables|Default|GetCan_Pick?)
    (Variables|Default|SetCan_Pick? false)
    (Physics|SetSimulatePhysics (Variables|Default|GetST_Fruits) true)
    (Variables|/Script/Engine.RotatingMovementComponent|SetRotationRate (Variables|Default|GetRotatingMovement) "0, 0, 0")
    (CallFunction|StopTime)))

(event EventTick
  (params (DeltaSeconds :type Float%20%28single-precision%29))
  (bind _returnvalue (Game|GetPlayerController 0))
  (bind (_locationx _locationy) (Game|Player|GetMousePosition _returnvalue))
  (bind _returnvalue_2 (Math|Vector2D|MakeVector2D _locationx _locationy))
  (bind (_worldposition _worlddirection) (Class|GameplayStatics|DeprojectScreentoWorld _returnvalue _returnvalue_2))
  (if (Variables|Default|GetCan_Pick?)
    (Transformation|SetActorLocation (+ _worldposition (* _worlddirection 1.5e+02)) false false)))

(event EventBeginPlay
  (bind _returnvalue (Viewport|GetViewportSize))
  (bind _fruits_array (Variables|Default|GetFruits_Array))
  (bind _st_fruits (Variables|Default|GetST_Fruits))
  (bind _returnvalue_2 (/ _returnvalue 2.0))
  (Variables|Default|SetRandom_FloatX (Math|Random|RandomFloatinRange -2e+02 2e+02))
  (Variables|Default|SetRandom_FloatY (Math|Random|RandomFloatinRange -5e+01 5e+01))
  (Variables|Default|SetSt_Index (Math|Random|RandomIntegerinRange 0 (Utilities|Array|LastIndex _fruits_array)))
  (Components|StaticMesh|SetStaticMesh (Variables|Default|GetST_Fruits) (Utilities|Array|Get(acopy) _fruits_array (Variables|Default|GetSt_Index)))
  (bind _新建轨迹_0 (Timeline|时间轴_0 Play)
    (:Update
      (Transformation|SetWorldLocation (Variables|Default|GetST_Fruits) (Math|Vector|Lerp(Vector) (Transformation|GetActorLocation) (+ (.WorldPosition (Class|GameplayStatics|DeprojectScreentoWorld (Game|GetPlayerController 0) (Math|Vector2D|MakeVector2D (+ (.x _returnvalue_2) (Variables|Default|GetRandom_FloatX)) (+ (.y _returnvalue_2) (Variables|Default|GetRandom_FloatY))))) (* (.WorldDirection (Class|GameplayStatics|DeprojectScreentoWorld (Game|GetPlayerController 0) (Math|Vector2D|MakeVector2D (+ (.x _returnvalue_2) (Variables|Default|GetRandom_FloatX)) (+ (.y _returnvalue_2) (Variables|Default|GetRandom_FloatY))))) 1e+02)) _新建轨迹_0) false false))
    (:Finished
      (Variables|/Script/Engine.RotatingMovementComponent|SetRotationRate (Variables|Default|GetRotatingMovement) "0, 0, 0")
      (Physics|SetSimulatePhysics _st_fruits true)
      (if (not (Math|Conversions|ToBoolean(Integer) (Math|Random|RandomIntegerinRange 0 1)))
        (Physics|AddImpulse _st_fruits (* (+ (.WorldPosition (Class|GameplayStatics|DeprojectScreentoWorld (Game|GetPlayerController 0) (Math|Vector2D|MakeVector2D (+ (.x _returnvalue_2) (Variables|Default|GetRandom_FloatX)) (+ (.y _returnvalue_2) (Variables|Default|GetRandom_FloatY))))) (* (.WorldDirection (Class|GameplayStatics|DeprojectScreentoWorld (Game|GetPlayerController 0) (Math|Vector2D|MakeVector2D (+ (.x _returnvalue_2) (Variables|Default|GetRandom_FloatX)) (+ (.y _returnvalue_2) (Variables|Default|GetRandom_FloatY))))) 1e+02)) 1.0) "None" false)
        (Utilities|FlowControl|Delay 2.0)
        (Actor|DestroyActor)))))

(event Input|MouseEvents|LeftMouseButton
  (params (Key :type Key%20Structure :default "None"))
  (:Released
    (bind _outactors (Actor|GetAllActorsOfClass "BP_FlyFruits_C"))
    (for _array_element _outactors
      (CallFunction|DropActor _array_element))))

(fn ConstructionScript)